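; StateTree task that moves a BP_ShootingTarget actor along a spline actor's path.
; On state entry it caches the cast target, then each tick sets the target's location from its stored DistanceTraveled along the spline.
; Distance grows by MovementSpeed per tick, without delta-time scaling.
; At the spline's end it resets the distance to zero and finishes the task successfully.
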(event `self.ReceiveLatentTick`
  (params (DeltaTime :type "Float (single-precision)"))
  (`Actor.K2_SetActorLocation` (`self.Actor`) (`SplineComponent.GetLocationAtDistanceAlongSpline` (`/Game/Blueprint/ST_Shooting/BP_SplineActor.Spline` (`self.SplineActor`)) (`/Game/Blueprint/ST_Shooting/BP_ShootingTarget.DistanceTraveled` (`self.As BP Shooting Target`)) "World") false false)
  (if (< (`/Game/Blueprint/ST_Shooting/BP_ShootingTarget.DistanceTraveled` (`self.As BP Shooting Target`)) (`SplineComponent.GetSplineLength` (`/Game/Blueprint/ST_Shooting/BP_SplineActor.Spline` (`self.SplineActor`))))
    (set `/Game/Blueprint/ST_Shooting/BP_ShootingTarget.DistanceTraveled` (+ (`/Game/Blueprint/ST_Shooting/BP_ShootingTarget.DistanceTraveled` (`self.As BP Shooting Target`)) (`self.MovementSpeed`)) (`self.As BP Shooting Target`))
    (else
      (set `/Game/Blueprint/ST_Shooting/BP_ShootingTarget.DistanceTraveled` 0.0 (`self.As BP Shooting Target`))
      (`self.FinishTask` true))))

(event `self.ReceiveLatentEnterState`
  (params (Transition :type "StateTreeTransitionResult Structure (by ref)"))
  (bind _asbp_shooting_target (cast `/Game/Blueprint/ST_Shooting/BP_ShootingTarget` (`self.Actor`)))
  (set `self.As BP Shooting Target` _asbp_shooting_target))