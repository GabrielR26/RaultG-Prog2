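; StateTree task that spins its context actor continuously while its state is active.
; On first entry it adds a RotatingMovementComponent to the actor at runtime with a fixed fast rotation rate and caches it.
; Later entries re-enable that component's tick, and exiting the state disables the tick to stop the spin without destroying the component.
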(event `self.ReceiveLatentEnterState`
  (params (Transition :type "StateTreeTransitionResult Structure (by ref)"))
  (`/Engine/EditorBlueprintResources/StandardMacros.IsValid` (`self.RotatingMovementComp`)
    (:`Is Valid`
      (`ActorComponent.SetComponentTickEnabled` (`self.RotatingMovementComp`) true))
    (:`Is Not Valid`
      (bind _returnvalue (`|AddComponentByClass` (`self.ContextActor`) "/Script/Engine.RotatingMovementComponent"))
      (bind _output_get (set `self.RotatingMovementComp` _returnvalue))
      (set `RotatingMovementComponent.RotationRate` (struct :`Yaw` 720.0) _output_get))))

(event `self.ReceiveExitState`
  (params (Transition :type "StateTreeTransitionResult Structure (by ref)"))
  (`ActorComponent.SetComponentTickEnabled` (`self.RotatingMovementComp`) false))